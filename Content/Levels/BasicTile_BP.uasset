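; BasicTile_BP is a level tile for an endless world, exposing its Arrow's world transform as the attach point.
; The player overlapping LockBarrier disables Barrier collision and turns it green.
; Leaving that volume restores collision, turns it red and asks InfinateWorld_GM to spawn a tile.
; The tile destroys itself when the player enters its DistroyTile volume.
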(event `self.ReceiveBeginPlay`)

(event `self.LockBarrier.OnComponentBeginOverlap`
  (params (OverlappedComponent :type "PrimitiveComponent Object Reference") (OtherActor :type "Actor Object Reference") (OtherComp :type "PrimitiveComponent Object Reference") (OtherBodyIndex :type Integer) (bFromSweep :type Boolean) (SweepResult :type "HitResult Structure (by ref)"))
  (`self.IsPlayer` OtherActor)
  (`self.UnLock`)
  (`PrimitiveComponent.SetMaterial` (`self.Barrier`) 0 "/Game/Levels/GreenBarrier.GreenBarrier"))

(event `self.LockBarrier.OnComponentEndOverlap`
  (params (OverlappedComponent :type "PrimitiveComponent Object Reference") (OtherActor :type "Actor Object Reference") (OtherComp :type "PrimitiveComponent Object Reference") (OtherBodyIndex :type Integer))
  (`self.IsPlayer` OtherActor)
  (`self.Lock`)
  (`PrimitiveComponent.SetMaterial` (`self.Barrier`) 0 "/Game/Levels/RedBarrier.RedBarrier")
  (bind _asinfinate_world_gm (cast `/Game/Levels/InfinateWorld_GM` (`GameplayStatics.GetGameMode` OtherActor)))
  (`/Game/Levels/InfinateWorld_GM.SpawnTile` _asinfinate_world_gm))

(event `self.DistroyTile.OnComponentBeginOverlap`
  (params (OverlappedComponent :type "PrimitiveComponent Object Reference") (OtherActor :type "Actor Object Reference") (OtherComp :type "PrimitiveComponent Object Reference") (OtherBodyIndex :type Integer) (bFromSweep :type Boolean) (SweepResult :type "HitResult Structure (by ref)"))
  (`self.IsPlayer` OtherActor)
  (`self.K2_DestroyActor`))

(fn `Get Attach Transform`
  (returns (`Attach Transform` :type "Transform Structure"))
  (return (`SceneComponent.K2_GetComponentToWorld` (`self.Arrow`))))

(fn `Lock`
  (`PrimitiveComponent.SetCollisionEnabled` (`self.Barrier`) "QueryAndPhysics"))

(fn `UnLock`
  (`PrimitiveComponent.SetCollisionEnabled` (`self.Barrier`) "NoCollision")
  (return))

(fn `UserConstructionScript`)