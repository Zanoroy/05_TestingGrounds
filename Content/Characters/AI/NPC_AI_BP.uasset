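; NPC_AI_BP is an AI controller Blueprint that drives a guard NPC through perception and a behavior tree.
; On BeginPlay it initializes the PatrolData blackboard, runs the GuardBehaviour tree and caches the blackboard component.
; AI Perception updates write sensed actors without the "Enemy" tag to the FocusActor key.
; A failed sense of such an actor clears that key, while Enemy-tagged actors are ignored.
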(event `self.ReceiveBeginPlay`
  (bind _blackboardcomponent (`self.UseBlackboard` "/Game/Characters/AI/BehaviourTree/PatrolData.PatrolData"))
  (`self.RunBehaviorTree` "/Game/Characters/AI/BehaviourTree/GuardBehaviour.GuardBehaviour")
  (set `self.BlackboardComp` _blackboardcomponent))

(event `self.ReceiveTick`
  (params (DeltaSeconds :type "Float (single-precision)")))

(event `self.AIPerception.OnTargetPerceptionUpdated`
  (params (Actor :type "Actor Object Reference") (Stimulus :type "AIStimulus Structure"))
  (bind _blackboardcomp (`self.BlackboardComp`))
  (if (`self.ActorHasTag` Actor "Enemy")
    _
    (elif (`.bSuccessfullySensed` (break `AIStimulus` Stimulus))
      (`BlackboardComponent.SetValueAsObject` _blackboardcomp "FocusActor" Actor)
      (else
        (`BlackboardComponent.ClearValue` _blackboardcomp "FocusActor")))))

(fn `UserConstructionScript`)