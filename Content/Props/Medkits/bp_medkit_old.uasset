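; Medkit pickup actor that restores a small amount of health to the player on contact.
; On overlap it checks for a player-controlled BP_Main_Character below full health, adds health clamped to the maximum, then destroys itself.
; BeginFocus and EndFocus toggle custom depth rendering on the Case, Locks and Handle components to mark focus.
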(event `self.ReceiveActorBeginOverlap`
  (params (OtherActor :type "Actor Object Reference"))
  (bind _asbp_main_character (cast `/Game/Characters/Main_Character/Behaviour/BP_Main_Character` OtherActor))
  (if (`Pawn.IsPlayerControlled` _asbp_main_character)
    (bind _health (`/Game/Characters/Main_Character/Behaviour/BP_Main_Character.Health` _asbp_main_character))
    (if (< _health 100.0)
      (set `/Game/Characters/Main_Character/Behaviour/BP_Main_Character.Health` (`KismetMathLibrary.FClamp` (+ _health 15.0) 0.0 100.0) _asbp_main_character)
      (`self.K2_DestroyActor`))))

(fn `BeginFocus`
  (`PrimitiveComponent.SetRenderCustomDepth` (`self.Case`) true)
  (`PrimitiveComponent.SetRenderCustomDepth` (`self.Locks`) true)
  (`PrimitiveComponent.SetRenderCustomDepth` (`self.Handle`) true))

(fn `EndFocus`
  (`PrimitiveComponent.SetRenderCustomDepth` (`self.Case`) false)
  (`PrimitiveComponent.SetRenderCustomDepth` (`self.Locks`) false)
  (`PrimitiveComponent.SetRenderCustomDepth` (`self.Handle`) false))

(fn `UserConstructionScript`)