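; BP_BasicTile is an infinite-world level tile that fills itself with props and AI enemies on BeginPlay.
; Enemy maximum follows TileNumber, bounded by MaxEnemy; zero MaxEnemy unlocks the barrier immediately.
; Player overlap with LockBarrier opens the barrier and counts the tile conquered once in InfinateWorld_GM; leaving relocks it.
; The DistroyTile trigger asks the game mode to spawn another tile, then destroys this one.
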(event `self.ReceiveBeginPlay`
  (bind _tilenumber (`self.TileNumber`))
  (bind _maxenemy (`self.MaxEnemy`))
  (`self.PlaceActors` "/Game/Geometry/Props/BP_Rock1.BP_Rock1_C" 2 4 201.0 1.0 1.5)
  (`self.PlaceActors` "/Game/Geometry/Props/BP_Rock2.BP_Rock2_C" 1 4 132.0 0.5 2.0)
  (`self.PlaceActors` "/Game/Geometry/Props/BP_Rock3.BP_Rock3_C" 0 2 175.0 0.5 1.5)
  (`self.PlaceActors` "/Game/Geometry/Props/BP_Sandbags.BP_Sandbags_C" 2 5 200.0 0.8)
  (`self.PlaceActors` "/Game/Geometry/Props/BP_Container_Broken.BP_Container_Broken_C" 1 3 306.0)
  (`self.PlaceActors` "/Game/Geometry/Props/BP_Container_Open.BP_Container_Open_C" 1 2 306.0)
  (`self.PlaceActors` "/Game/Geometry/Props/BP_Box.BP_Box_C" 2 5 64.0 1.0 2.0)
  (if (== (`self.MaxEnemy`) 0)
    (`self.UnLock`)
    (else
      (`self.PlaceAIPawn` "/Game/Characters/Main_Character/Behaviour/BP_Main_Character.BP_Main_Character_C" (`self.MinEnemy`) (`KismetMathLibrary.Clamp` (select `bool` (< _tilenumber _maxenemy) :`false` _maxenemy :`true` _tilenumber) 2 _maxenemy) 64.0))))

(event `self.LockBarrier.OnComponentBeginOverlap`
  (params (OverlappedComponent :type "PrimitiveComponent Object Reference") (OtherActor :type "Actor Object Reference") (OtherComp :type "PrimitiveComponent Object Reference") (OtherBodyIndex :type Integer) (bFromSweep :type Boolean) (SweepResult :type "HitResult Structure (by ref)"))
  (`self.IsPlayer` OtherActor)
  (`self.UnLock`)
  (`self.TileConquered`))

(event `self.LockBarrier.OnComponentEndOverlap`
  (params (OverlappedComponent :type "PrimitiveComponent Object Reference") (OtherActor :type "Actor Object Reference") (OtherComp :type "PrimitiveComponent Object Reference") (OtherBodyIndex :type Integer))
  (`self.IsPlayer` OtherActor)
  (`self.Lock`))

(event `self.DistroyTile.OnComponentBeginOverlap`
  (params (OverlappedComponent :type "PrimitiveComponent Object Reference") (OtherActor :type "Actor Object Reference") (OtherComp :type "PrimitiveComponent Object Reference") (OtherBodyIndex :type Integer) (bFromSweep :type Boolean) (SweepResult :type "HitResult Structure (by ref)"))
  (`self.IsPlayer` OtherActor)
  (bind _asinfinate_world_gm (cast `/Game/GameModes/InfinateWorld_GM` (`GameplayStatics.GetGameMode` OtherActor)))
  (`/Game/GameModes/InfinateWorld_GM.SpawnTile` _asinfinate_world_gm)
  (`self.K2_DestroyActor`))

(fn `Get Attach Transform`
  (returns (`Attach Transform` :type "Transform Structure"))
  (return (`SceneComponent.K2_GetComponentToWorld` (`self.Arrow`))))

(fn `Lock`
  (bind _barrier (`self.Barrier`))
  (`PrimitiveComponent.SetCollisionEnabled` _barrier "QueryAndPhysics")
  (`PrimitiveComponent.SetMaterial` _barrier 0 "/Game/Materials/MI_Barrier_Red.MI_Barrier_Red"))

(fn `TileConquered`
  (if (not (`self.IsTileConquered`))
    (set `self.IsTileConquered` true)
    (bind _asinfinate_world_gm (cast `/Game/GameModes/InfinateWorld_GM` (`GameplayStatics.GetGameMode`)))
    (set `/Game/GameModes/InfinateWorld_GM.TilesConquered` (+ (`/Game/GameModes/InfinateWorld_GM.TilesConquered` _asinfinate_world_gm) 1) _asinfinate_world_gm)))

(fn `UnLock`
  (bind _barrier (`self.Barrier`))
  (`PrimitiveComponent.SetCollisionEnabled` _barrier "NoCollision")
  (`PrimitiveComponent.SetMaterial` _barrier 0 "/Game/Materials/MI_Barrier_Green.MI_Barrier_Green")
  (return))

(fn `UserConstructionScript`)